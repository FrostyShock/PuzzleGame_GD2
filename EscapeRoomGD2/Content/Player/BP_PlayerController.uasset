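; Player controller for a first-person puzzle game, handling movement, interaction, object inspection, minigames and the notes UI.
; A short view-direction trace finds BPI_PuzzleGame actors, whose returned interaction type selects pickup inspection, a keypad or chessboard minigame, dialogue or a collectible note.
; Inspected objects ease to the player's view anchor for rotation, while chessboard play blends the camera and forwards cursor grabs through messages.
; Each mode swaps Enhanced Input mapping contexts, input mode and cursor visibility.
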(event `EnhancedInput|/Game/Data/Input/Chessboard/IA_Exit`
  (params (ActionValue :type Boolean) (ElapsedSeconds :type "Float (double-precision)") (TriggeredSeconds :type "Float (double-precision)") (InputAction :type "InputAction Object Reference" :default "/Game/Data/Input/Chessboard/IA_Exit.IA_Exit"))
  (:`Started`
    (`self.SetViewTargetWithBlend` (`self.DefaultPlayerRef`) 0.5)
    (`KismetSystemLibrary.Delay` 0.5)
    (`self.Default Player Map Change`)))

(event `EnhancedInput|/Game/Data/Input/Chessboard/IA_Reset`
  (params (ActionValue :type Boolean) (ElapsedSeconds :type "Float (double-precision)") (TriggeredSeconds :type "Float (double-precision)") (InputAction :type "InputAction Object Reference" :default "/Game/Data/Input/Chessboard/IA_Reset.IA_Reset"))
  (bind _testedactor (`self.TestedActor`))
  (:`Started`
    (`/Engine/EditorBlueprintResources/StandardMacros.IsValid` _testedactor
      (:`Is Valid`
        (message `/Game/Data/Interfaces/BPI_PuzzleGame.On Reset` _testedactor)))))

(event `Chessboard Camera Setter`
  (`self.SetViewTargetWithBlend` (`self.TestedActor`) 1.0))

(event `EnhancedInput|/Game/Data/Input/Chessboard/IA_Grab`
  (params (ActionValue :type Boolean) (ElapsedSeconds :type "Float (double-precision)") (TriggeredSeconds :type "Float (double-precision)") (InputAction :type "InputAction Object Reference" :default "/Game/Data/Input/Chessboard/IA_Grab.IA_Grab"))
  (bind (_bblockinghit _binitialoverlap _time _distance _location _impactpoint _normal _impactnormal _physmat _hitactor _hitcomponent) (`GameplayStatics.BreakHitResult` (`self.GetHitResultUnderCursorByChannel` "TraceTypeQuery1")))
  (:`Triggered`
    (message `/Game/Data/Interfaces/BPI_PuzzleGame.Send Cursor Location` _hitactor (`.Location` (`GameplayStatics.BreakHitResult` (`self.GetHitResultUnderCursorForObjects` (`self.Cursor Detection`))))))
  (:`Started`
    (message `/Game/Data/Interfaces/BPI_PuzzleGame.On Pickup` _hitactor _hitcomponent))
  (:`Canceled`
    (message `/Game/Data/Interfaces/BPI_PuzzleGame.On Release` _hitactor _hitcomponent :!label _label))
  (:`Completed`
    (goto _label)))

(event `Minigame Interaction`
  (params (`Interactable Actor` :type "Actor Object Reference"))
  ; Interaction Input Handler
  ;; Object selection handler
  (if (== (`GameplayStatics.GetObjectClass` `Interactable Actor`) "/Game/Blueprints/PuzzleObjects/BP_Keypad.BP_Keypad_C")
    (`self.UI ONLY MAP CHANGE`)
    (else
      (set `self.playerNormalTransform` (`self.GetTransform` (`GameplayStatics.GetPlayerPawn` 0)))
      (`self.Chessboard Camera Setter`)
      (`self.ChessBoard MAP CHANGE`))))

(event `Inspection Interaction`
  (params (`Interacting Actor` :type "Actor Object Reference"))
  (bind _held_object (`self.Held Object`))
  ; Inspection Lerp Interaction
  (set `self.Held Object` `Interacting Actor`)
  (set `self.Holding Object` true)
  (`self.Inspection Player Map Change`)
  (bind (_direction _lerp_value) (`Timeline|Grab Interp Timeline` :!via `PlayFromStart`)
    (:`Update`
      (`/Engine/EditorBlueprintResources/StandardMacros.IsValid` _held_object
        (:`Is Valid`
          (bind (_returnvalue_location _returnvalue_rotation _returnvalue_scale) (`KismetMathLibrary.BreakTransform` (`KismetMathLibrary.TLerp` (`self.GetTransform` (`self.Held Object`)) (`SceneComponent.K2_GetComponentToWorld` (`/Game/Player/BP_DefaultPlayer.ViewAnchor` (`self.DefaultPlayerRef`))) _lerp_value)))
          (`self.K2_SetActorTransform` _held_object (`KismetMathLibrary.MakeTransform` _returnvalue_location _returnvalue_rotation _returnvalue_scale) false true)
          (`self.K2_AttachToComponent` (`self.Held Object`) (`/Game/Player/BP_DefaultPlayer.ViewAnchor` (`self.DefaultPlayerRef`)) "None" "KeepWorld" "KeepRelative" "KeepRelative" false))))))

(event `EnhancedInput|/Game/Data/Input/Default/IA_Interaction`
  (params (ActionValue :type Boolean) (ElapsedSeconds :type "Float (double-precision)") (TriggeredSeconds :type "Float (double-precision)") (InputAction :type "InputAction Object Reference" :default "/Game/Data/Input/Default/IA_Interaction.IA_Interaction"))
  (bind _ui_ref (`self.UI Ref`))
  (bind _wid_textinfo (`/Game/UI/WID_UserInterface.WID_TextInfo` _ui_ref))
  ; Interaction Input Handler
  (:`Started`
    (if (`self.Holding Object`)
      (`self.Release Object`)
      (`/Game/UI/WID_UserInterface.Hide Item Info` (`self.UI Ref`))
      (else
        (bind _outhit (`self.Interaction Function`))
        (bind (_bblockinghit _binitialoverlap _time _distance _location _impactpoint _normal _impactnormal _physmat _hitactor _hitcomponent) (`GameplayStatics.BreakHitResult` _outhit))
        (if (`KismetSystemLibrary.DoesImplementInterface` _hitactor "/Game/Data/Interfaces/BPI_PuzzleGame.BPI_PuzzleGame_C")
          (bind (_interactable_actor _interaction_type _iteminfo) (message `/Game/Data/Interfaces/BPI_PuzzleGame.OnInteracted` _hitactor _hitcomponent))
          (set `self.TestedActor` _interactable_actor)
          ;; Object selection handler
          (switch `/Game/Data/Enums/Enum_InteractionType` _interaction_type
            (:`NewEnumerator0`
              (if (`self.Inspecting`)
                (`self.Inspection Interaction` _interactable_actor)
                (set `/Game/UI/WID_TextInfo.ItemInfo` _iteminfo _wid_textinfo)
                (`/Game/UI/WID_UserInterface.Display Item Info` _ui_ref)))
            (:`NewEnumerator1`
              (`self.Minigame Interaction` (`self.TestedActor`)))
            (:`NewEnumerator2`
              (`self.Inspection Player Map Change`))
            (:`NewEnumerator4`
              (`self.Inspection Interaction` _interactable_actor)
              (bind _output_get (set `/Game/UI/WID_TextInfo.ItemInfo` _iteminfo _wid_textinfo))
              (`/Game/UI/WID_NotesPanel.Add New Entry` (`/Game/UI/WID_UserInterface.WID_NotesPanel` _ui_ref) _output_get)
              (`/Game/UI/WID_UserInterface.Display Item Info` _ui_ref)
              (`/Engine/EditorBlueprintResources/StandardMacros.DoOnce` false
                (:`Completed`
                  (`/Game/UI/WID_UserInterface.Show Notes Tooltip` (`self.UI Ref`)))))))))))

(event `EnhancedInput|/Game/Data/Input/Default/IA_Notes`
  (params (ActionValue :type Boolean) (ElapsedSeconds :type "Float (double-precision)") (TriggeredSeconds :type "Float (double-precision)") (InputAction :type "InputAction Object Reference" :default "/Game/Data/Input/Default/IA_Notes.IA_Notes"))
  (bind _wid_notespanel (`/Game/UI/WID_UserInterface.WID_NotesPanel` (`self.UI Ref`)))
  ; Notes UI Handler
  (:`Started`
    (if (not (`KismetArrayLibrary.Array_IsEmpty` (`/Game/UI/WID_NotesPanel.ButtonArray` (`/Game/UI/WID_UserInterface.WID_NotesPanel` (`self.UI Ref`)))))
      (`/Engine/EditorBlueprintResources/StandardMacros.FlipFlop`
        (:`A`
          (`Widget.SetVisibility` _wid_notespanel "Visible")
          (`WidgetBlueprintLibrary.SetInputMode_GameAndUIEx` self (`self.UI Ref`))
          (set `self.bShowMouseCursor` true)
          (set `self.Inspecting` true))
        (:`B`
          (`Widget.SetVisibility` _wid_notespanel "Hidden")
          (`WidgetBlueprintLibrary.SetInputMode_GameOnly` self)
          (set `self.bShowMouseCursor` false)
          (set `self.Inspecting` true))))))

(event `Release Object`
  ; Release Object
  (`self.Default Player Map Change`)
  (`self.K2_DetachFromActor` (`self.Held Object`) "KeepWorld" "KeepWorld" "KeepRelative")
  (message `/Game/Data/Interfaces/BPI_PuzzleGame.OnInteracted` (`self.Held Object`) null)
  (set `self.Holding Object` false))

(event `Create UI Container`
  (bind _returnvalue (`|CreateWidget` "/Game/UI/WID_UserInterface.WID_UserInterface_C"))
  (bind _output_get (set `self.UI Ref` _returnvalue))
  (`UserWidget.AddToViewport` _output_get 0))

(event `Default Player Map Change`
  (bind _returnvalue (pcsubsystem `EnhancedInputLocalPlayerSubsystem` self))
  ; Input Map Handlers
  (`EnhancedInputSubsystemInterface.ClearAllMappings` _returnvalue)
  (message `EnhancedInputSubsystemInterface.AddMappingContext` _returnvalue "/Game/Data/Input/Default/IMC_Default.IMC_Default" 0 (struct))
  (`WidgetBlueprintLibrary.SetInputMode_GameOnly` self)
  (set `self.bShowMouseCursor` false)
  (set `self.Inspecting` false))

(event `self.ReceiveBeginPlay`
  (add `self.OnPossessedPawnChanged` (delegate `OnPossessedPawnChanged_Event`))
  (`self.Default Player Map Change`)
  (bind _asbp_default_player (cast `/Game/Player/BP_DefaultPlayer` (`GameplayStatics.GetPlayerPawn` 0)))
  (set `self.DefaultPlayerRef` _asbp_default_player)
  (`self.Create UI Container`))

(event `EnhancedInput|/Game/Data/Input/Default/IA_Look`
  (params (ActionValue :type "Vector2D Structure") (ElapsedSeconds :type "Float (double-precision)") (TriggeredSeconds :type "Float (double-precision)") (InputAction :type "InputAction Object Reference" :default "/Game/Data/Input/Default/IA_Look.IA_Look"))
  ; Default Inputs
  (:`Triggered`
    (`self.Look Function` ActionValue)))

(event `Inspection Player Map Change`
  (bind (_x _y) (`KismetMathLibrary.BreakVector2D` (`WidgetLayoutLibrary.GetViewportSize`)))
  (bind _returnvalue (pcsubsystem `EnhancedInputLocalPlayerSubsystem` self))
  ; Input Map Handlers
  (`EnhancedInputSubsystemInterface.ClearAllMappings` _returnvalue)
  (message `EnhancedInputSubsystemInterface.AddMappingContext` _returnvalue "/Game/Data/Input/Inspection/IMC_Inspection.IMC_Inspection" 0 (struct))
  (`self.SetMouseLocation` (`KismetMathLibrary.FTrunc` (/ _x 2.0)) (`KismetMathLibrary.FTrunc` (/ _y 2.0)))
  (`WidgetBlueprintLibrary.SetInputMode_GameAndUIEx` self (`self.UI Ref`))
  (set `self.bShowMouseCursor` true)
  (set `self.Inspecting` true))

(event `OnPossessedPawnChanged_Event` :!signature `self.OnPossessedPawnChanged`
  (params (OldPawn :type "Pawn Object Reference") (NewPawn :type "Pawn Object Reference"))
  (bind _pawn_enum (message `/Game/Data/Interfaces/BPI_PuzzleGame.OnPawnChanged` NewPawn))
  (switch `/Game/Data/Enums/Enum_PossessedPawn` _pawn_enum
    (:`NewEnumerator0`
      (`self.Default Player Map Change`))))

(event `EnhancedInput|/Game/Data/Input/Default/IA_Movement`
  (params (ActionValue :type "Vector2D Structure") (ElapsedSeconds :type "Float (double-precision)") (TriggeredSeconds :type "Float (double-precision)") (InputAction :type "InputAction Object Reference" :default "/Game/Data/Input/Default/IA_Movement.IA_Movement"))
  ; Default Inputs
  (:`Triggered`
    (`self.Movement Function` ActionValue)))

(event `UI ONLY MAP CHANGE`
  (bind (_x _y) (`KismetMathLibrary.BreakVector2D` (`WidgetLayoutLibrary.GetViewportSize`)))
  (bind _returnvalue (pcsubsystem `EnhancedInputLocalPlayerSubsystem` self))
  ; Input Map Handlers
  (`EnhancedInputSubsystemInterface.ClearAllMappings` _returnvalue)
  (message `EnhancedInputSubsystemInterface.AddMappingContext` _returnvalue "/Game/Data/Input/Inspection/IMC_Inspection.IMC_Inspection" 0 (struct))
  (`self.SetMouseLocation` (`KismetMathLibrary.FTrunc` (/ _x 2.0)) (`KismetMathLibrary.FTrunc` (/ _y 2.0)))
  (`WidgetBlueprintLibrary.SetInputMode_UIOnlyEx` self null)
  (set `self.bShowMouseCursor` true)
  (set `self.Inspecting` true))

(event `EnhancedInput|/Game/Data/Input/Inspection/IA_Rotate`
  (params (ActionValue :type "Vector2D Structure") (ElapsedSeconds :type "Float (double-precision)") (TriggeredSeconds :type "Float (double-precision)") (InputAction :type "InputAction Object Reference" :default "/Game/Data/Input/Inspection/IA_Rotate.IA_Rotate"))
  (bind (_x _y) (`KismetMathLibrary.BreakVector2D` ActionValue))
  (bind _held_object (`self.Held Object`))
  ; Rotation Input
  (:`Triggered`
    (`/Engine/EditorBlueprintResources/StandardMacros.IsValid` (`self.Held Object`)
      (:`Is Valid`
        (`self.K2_AddActorWorldRotation` _held_object (`KismetMathLibrary.RotatorFromAxisAndAngle` (0.0 0.0 1.0) (* _x 1.0)) false false)
        (`self.K2_AddActorWorldRotation` _held_object (`KismetMathLibrary.RotatorFromAxisAndAngle` (`KismetMathLibrary.Normal` (`KismetMathLibrary.Cross_VectorVector` (`SceneComponent.GetForwardVector` (`/Game/Player/BP_DefaultPlayer.Camera` (`self.DefaultPlayerRef`))) (0.0 0.0 1.0))) (* _y 1.0)) false false)))))

(event `ChessBoard MAP CHANGE`
  (bind _returnvalue (pcsubsystem `EnhancedInputLocalPlayerSubsystem` self))
  (`EnhancedInputSubsystemInterface.ClearAllMappings` _returnvalue)
  (message `EnhancedInputSubsystemInterface.AddMappingContext` _returnvalue "/Game/Data/Input/Chessboard/IMC_ChessBoard.IMC_ChessBoard" 0 (struct))
  (`WidgetBlueprintLibrary.SetInputMode_GameAndUIEx` self null "DoNotLock" false)
  (`GameplayStatics.SetViewportMouseCaptureMode` "CaptureDuringMouseDown")
  (set `self.bShowMouseCursor` true)
  (set `self.Inspecting` true))

(event `self.ReceiveTick`
  (params (DeltaSeconds :type "Float (single-precision)")))

(fn `Interaction Function`
  (returns (OutHit :type "HitResult Structure"))
  (bind _returnvalue (`GameplayStatics.GetPlayerPawn` 0))
  (bind _x (.x (`self.K2_GetActorLocation` _returnvalue)))
  (bind _y (.y (`self.K2_GetActorLocation` _returnvalue)))
  (bind _z (.z (`self.K2_GetActorLocation` _returnvalue)))
  (bind _outhit (`KismetSystemLibrary.LineTraceSingle` :`Start` (`KismetMathLibrary.MakeVector` _x _y (+ 70.0 _z)) :`End` (`KismetMathLibrary.MakeVector` (+ _x (.x (* (`KismetMathLibrary.Conv_RotatorToVector` (`Pawn.GetControlRotation` _returnvalue)) 350.0))) (+ _y (.y (* (`KismetMathLibrary.Conv_RotatorToVector` (`Pawn.GetControlRotation` _returnvalue)) 350.0))) (+ _z (+ 70.0 (.z (* (`KismetMathLibrary.Conv_RotatorToVector` (`Pawn.GetControlRotation` _returnvalue)) 350.0))))) :`TraceChannel` "TraceTypeQuery1" :`DrawTime` 1.5))
  (return _outhit))

(fn `Look Function`
  (params (`Action Value` :type "Vector2D Structure"))
  (bind (_x _y) (`KismetMathLibrary.BreakVector2D` `Action Value`))
  (bind _returnvalue (`GameplayStatics.GetPlayerPawn` 0))
  (`Pawn.AddControllerPitchInput` _returnvalue _y)
  (`Pawn.AddControllerYawInput` _returnvalue _x))

(fn `Movement Function`
  (params (`Action Value` :type "Vector2D Structure"))
  (bind (_x _y) (`KismetMathLibrary.BreakVector2D` `Action Value`))
  (bind _returnvalue (`GameplayStatics.GetPlayerPawn` 0))
  (bind _returnvalue_2 (`Pawn.GetMovementComponent` _returnvalue))
  (`PawnMovementComponent.AddInputVector` _returnvalue_2 (* _y (`self.GetActorForwardVector` _returnvalue)) false)
  (`PawnMovementComponent.AddInputVector` _returnvalue_2 (* _x (`self.GetActorRightVector` _returnvalue)) false))

(fn `UserConstructionScript`)