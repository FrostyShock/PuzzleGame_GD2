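; BP_Light1 is a light actor with a spotlight that can flicker at random during play.
; On BeginPlay, if the Flicker flag is set, it starts a fast looping timer bound to the LightFlicker event.
; Each timer tick rolls a random integer, setting the spotlight to the flicker brightness on one outcome and back to normal brightness otherwise.
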(event `self.ReceiveBeginPlay`
  (if (`self.Flicker`)
    (`KismetSystemLibrary.K2_SetTimerDelegate` (delegate `Light Flicker`) 0.1 true)))

(event `Light Flicker`
  (bind _spotlight (`self.SpotLight`))
  (switch `int` (`KismetMathLibrary.RandomIntegerInRange` 0 10)
    (:`Default`
      (`LightComponent.SetIntensity` _spotlight (`self.NormalBrightness`)))
    (:`0`
      (`LightComponent.SetIntensity` _spotlight (`self.FlickerBrightness`)))))

(fn `UserConstructionScript`)