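; Interactable keypad puzzle actor that shows a PIN pad interface and can open a linked door.
; Interacting calls OpenKeypad, which creates WID_PinPad for the first player controller, passes itself as KeyPadRef and adds the widget to the viewport.
; A separate OpenDoor event, not called within this Blueprint, forwards to DoorRef when that reference is valid.
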(event `Open Keypad`
  (bind _returnvalue (`|CreateWidget` "/Game/UI/WID_PinPad.WID_PinPad_C" (`GameplayStatics.GetPlayerController` 0) self))
  (`UserWidget.AddToViewport` _returnvalue 0))

(event `Open Door`
  (bind _door_ref (`self.Door Ref`))
  (`/Engine/EditorBlueprintResources/StandardMacros.IsValid` _door_ref
    (:`Is Valid`
      (`/Game/Blueprints/PuzzleObjects/BP_Door.Open Door` _door_ref))))

(fn `OnInteracted`
  (params (`Component Hit` :type "PrimitiveComponent Object Reference"))
  (returns (`Interactable Actor` :type "Actor Object Reference") (`Interaction Type` :type "/Game/Data/Enums/Enum_InteractionType Enum") (ItemInfo :type "/Game/Data/ItemData/STR_ItemInfo Structure"))
  (`self.Open Keypad`)
  (return self (`self.Interaction Type`)))

(fn `OnPawnChanged`
  (returns (`Pawn Enum` :type "/Game/Data/Enums/Enum_PossessedPawn Enum"))
  (return "NewEnumerator0"))

(fn `UserConstructionScript`)