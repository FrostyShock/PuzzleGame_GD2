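; Puzzle actor that creates an infinite hallway illusion by teleporting whatever enters its two trigger boxes.
; Each box converts the overlap's sweep location into its local space and reapplies it at its paired target, preserving relative position but setting only location.
; Teleports fire only when the sweep normal matches a hardcoded world-space direction, making them one-way and orientation-dependent.
; The first box accepts only the player pawn, while the second moves any actor.
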(event `self.First Box.OnComponentBeginOverlap`
  (params (OverlappedComponent :type "PrimitiveComponent Object Reference") (OtherActor :type "Actor Object Reference") (OtherComp :type "PrimitiveComponent Object Reference") (OtherBodyIndex :type Integer) (bFromSweep :type Boolean) (SweepResult :type "HitResult Structure (by ref)"))
  (bind (_bblockinghit _binitialoverlap _time _distance _location _impactpoint _normal) (`GameplayStatics.BreakHitResult` SweepResult))
  (if (and (== OtherActor (`GameplayStatics.GetPlayerPawn` 0)) (== _normal (0.0 -1.0 0.0) :`ErrorTolerance` 0.1))
    (`/Engine/EditorBlueprintResources/StandardMacros.IsValid` OtherActor
      (:`Is Valid`
        (`self.K2_SetActorLocation` OtherActor (`KismetMathLibrary.TransformLocation` (`SceneComponent.K2_GetComponentToWorld` (`self.First Box Target`)) (`KismetMathLibrary.InverseTransformLocation` (`SceneComponent.K2_GetComponentToWorld` (`self.First Box`)) _location)) false true)))))

(event `self.Second Box.OnComponentBeginOverlap`
  (params (OverlappedComponent :type "PrimitiveComponent Object Reference") (OtherActor :type "Actor Object Reference") (OtherComp :type "PrimitiveComponent Object Reference") (OtherBodyIndex :type Integer) (bFromSweep :type Boolean) (SweepResult :type "HitResult Structure (by ref)"))
  (bind (_bblockinghit _binitialoverlap _time _distance _location _impactpoint _normal) (`GameplayStatics.BreakHitResult` SweepResult))
  (if (== _normal (-1.0 -0.0 0.0) :`ErrorTolerance` 0.1)
    (`self.K2_SetActorLocation` OtherActor (`KismetMathLibrary.TransformLocation` (`SceneComponent.K2_GetComponentToWorld` (`self.Second Box Target`)) (`KismetMathLibrary.InverseTransformLocation` (`SceneComponent.K2_GetComponentToWorld` (`self.Second Box`)) _location)) false true)))

(fn `UserConstructionScript`)