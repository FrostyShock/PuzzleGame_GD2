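; BP_PerspOverlap is a puzzle trigger that detects when the player views the scene from a specific spot and angle.
; Player pawn overlap starts a fast looping timer, apparently driving CheckPlayerOrientation, with no logic to stop it.
; The check compares control rotation's quaternion XYZ and pawn location against hard-coded targets within tolerances.
; When both match, it sets PerspClue on the GI_Default game instance.
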(event `self.ReceiveActorBeginOverlap`
  (params (OtherActor :type "Actor Object Reference"))
  (if (== OtherActor (`GameplayStatics.GetPlayerPawn` 0))
    (`KismetSystemLibrary.K2_SetTimerDelegate` (`|CreateDelegate` :!event `CheckPlayerOrientation`) 0.07 true true)))

(event `CheckPlayerOrientation`
  (bind _returnvalue (`GameplayStatics.GetPlayerPawn` 0))
  (bind (_x _y _z) (`KismetMathLibrary.BreakQuat` (`KismetMathLibrary.Conv_RotatorToQuaternion` (`Pawn.GetControlRotation` _returnvalue))))
  (if (and (== (`KismetMathLibrary.MakeVector` _x _y _z) (`KismetMathLibrary.MakeVector` 0.064 0.069 0.679) :`ErrorTolerance` 0.2) (== (`self.K2_GetActorLocation` _returnvalue) (-314.0 2257.0 -388.0) :`ErrorTolerance` 50.0))
    (bind _asgi_default (cast `/Game/Levels/LevelData/GI_Default` (`GameplayStatics.GetGameInstance`)))
    (set `/Game/Levels/LevelData/GI_Default.PerspClue` true _asgi_default)))

(fn `UserConstructionScript`)