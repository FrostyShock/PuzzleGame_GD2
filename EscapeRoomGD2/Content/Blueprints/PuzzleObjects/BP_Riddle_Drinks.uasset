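; BP_Riddle_Drinks is an interactable puzzle object that unlocks the clue flag for the first riddle.
; Its OnInteracted function calls Interacted, then casts the game instance to GI_Default and sets Riddle1Clue, keeping that progress in the game instance.
; It returns itself, a fixed interaction type and its ItemInfo to the caller.
; The event graph holds only disabled default events.
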(fn `OnInteracted`
  (params (`Component Hit` :type "PrimitiveComponent Object Reference"))
  (returns (`Interactable Actor` :type "Actor Object Reference") (`Interaction Type` :type "/Game/Data/Enums/Enum_InteractionType Enum") (ItemInfo :type "/Game/Data/ItemData/STR_ItemInfo Structure"))
  (`self.Interacted`)
  (bind _asgi_default (cast `/Game/Levels/LevelData/GI_Default` (`GameplayStatics.GetGameInstance`)))
  (set `/Game/Levels/LevelData/GI_Default.Riddle1Clue` true _asgi_default)
  (return self "NewEnumerator4" (`self.ItemInfo`)))

(fn `UserConstructionScript`
  (`parent.UserConstructionScript`))