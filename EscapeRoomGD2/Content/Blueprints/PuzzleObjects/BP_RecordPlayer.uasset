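; BP_RecordPlayer is an interactable record player puzzle whose drawer reveals a puzzle piece when solved.
; Cranking animates via timeline; once the Game Instance has MorseCodeNote, it shows and spins the record, plays audio and advances a wrapping dial pointer.
; Pressing the dial or pointer at the correct crank count slides the drawer open, otherwise it resets count and playback.
; Focus highlights controls through custom depth; disconnected win-screen nodes never run.
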(event `Open Drawer`
  ; Temp END OF GAME
  (`SceneComponent.SetVisibility` (`self.PuzzlePiece`) true false)
  (`AudioComponent.Stop` (`self.Audio`))
  (bind (_direction _rotate) (`Timeline|DrawerTimeline` :!via `PlayFromStart`)
    (:`Update`
      (`SceneComponent.K2_SetRelativeLocation` (`self.Drawer`) (`KismetMathLibrary.MakeVector` 0.0 _rotate) false false))
    (:`Finished`
      (set `self.Puzzle Complete` true))))

(event `self.ReceiveBeginPlay`
  (`MovementComponent.SetUpdatedComponent` (`self.RotatingMovement`) (`self.Record`)))

(event `/Game/Data/Interfaces/BPI_PuzzleGame.On Focused`
  (params (Focused :type Boolean) (Component :type "PrimitiveComponent Object Reference"))
  (if (or (== Component (`self.Dial`)) (== Component (`self.Pointer`)) (== Component (`self.Crank`)))
    (`PrimitiveComponent.SetRenderCustomDepth` Component Focused)))

(event `Play Record`
  (if (not (`self.Audio Playing`))
    (`AudioComponent.Play` (`self.Audio`) 0.0)
    (`ActorComponent.Activate` (`self.RotatingMovement`) false)
    (set `self.Audio Playing` true)))

(event `Interacted`
  (params (`Component Interacted` :type "PrimitiveComponent Object Reference"))
  (bind _pointer (`self.Pointer`))
  (if (or (== `Component Interacted` (`self.Dial`)) (== `Component Interacted` (`self.Pointer`)))
    (if (== (`self.CrankCount`) 4)
      (`self.Open Drawer`)
      (else
        (set `self.CrankCount` 0)
        (`SceneComponent.K2_SetRelativeRotation` (`self.Pointer`) (struct :`Yaw` 10.0) false false)
        (`AudioComponent.Stop` (`self.Audio`))))
    (set `self.Audio Playing` false)
    (`ActorComponent.Deactivate` (`self.RotatingMovement`))
    (elif (not (`self.Puzzle Complete`))
      (bind _asgi_default (cast `/Game/Levels/LevelData/GI_Default` (`GameplayStatics.GetGameInstance`)))
      (if (`/Game/Levels/LevelData/GI_Default.MorseCodeNote` _asgi_default)
        (`SceneComponent.SetVisibility` (`self.Record`) true false))
      (`/Engine/EditorBlueprintResources/StandardMacros.DoOnce` false :!label _label
        (:`Completed`
          (bind (_direction _rotate) (`Timeline|Timeline` :!via `PlayFromStart`)
            (:`Update`
              (`SceneComponent.K2_SetRelativeRotation` (`self.Scene`) (`KismetMathLibrary.MakeRotator` _rotate) false false))
            (:`Finished`
              (bind _asgi_default_2 (cast `/Game/Levels/LevelData/GI_Default` (`GameplayStatics.GetGameInstance`)))
              (if (`/Game/Levels/LevelData/GI_Default.MorseCodeNote` _asgi_default_2)
                (`self.Play Record`)
                (bind _result (`/Engine/EditorBlueprintResources/StandardMacros.IncrementInt` (`self.CrankCount`))
                  (:`  `
                    (if (== _result 10)
                      (set `self.CrankCount` 0)
                      (`SceneComponent.K2_SetRelativeRotation` _pointer (struct :`Yaw` 10.0) false false)
                      (goto _label :!via `Reset`)
                      (else
                        (`SceneComponent.K2_AddRelativeRotation` _pointer (struct :`Yaw` 38.0) false false)
                        (goto _label :!via `Reset`)))))
                (else
                  (goto _label :!via `Reset`))))))))))

(fn `OnInteracted`
  (params (`Component Hit` :type "PrimitiveComponent Object Reference"))
  (returns (`Interactable Actor` :type "Actor Object Reference") (`Interaction Type` :type "/Game/Data/Enums/Enum_InteractionType Enum") (ItemInfo :type "/Game/Data/ItemData/STR_ItemInfo Structure"))
  (`self.Interacted` `Component Hit`)
  (return self "NewEnumerator5"))

(fn `OnPawnChanged`
  (returns (`Pawn Enum` :type "/Game/Data/Enums/Enum_PossessedPawn Enum"))
  (return "NewEnumerator0"))

(fn `UserConstructionScript`)