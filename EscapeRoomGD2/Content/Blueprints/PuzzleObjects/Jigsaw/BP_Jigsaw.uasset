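; BP_Jigsaw is an interactable jigsaw puzzle that rewards collected pieces with a chest key in a drawer.
; On interaction it reads two piece flags from GI_Default and reveals the matching KeyPiece meshes.
; With both pieces it also shows ChestKey and runs OpenDrawer, a one-shot timeline that slides Box along Y.
; Focusing toggles custom depth on the focused component for highlighting.
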(event `/Game/Data/Interfaces/BPI_PuzzleGame.On Focused`
  (params (Focused :type Boolean) (Component :type "PrimitiveComponent Object Reference"))
  (`PrimitiveComponent.SetRenderCustomDepth` Component Focused))

(event `Interacted`
  (bind _keypiece1 (`self.keyPiece1`))
  (bind _keypiece2 (`self.keyPiece2`))
  (bind _keypiece2_2 (`self.keyPiece2`))
  (bind _asgi_default (cast `/Game/Levels/LevelData/GI_Default` (`GameplayStatics.GetGameInstance`)))
  (bind _puzzlepiece1 (`/Game/Levels/LevelData/GI_Default.PuzzlePiece1` _asgi_default))
  (bind _puzzlepiece2 (`/Game/Levels/LevelData/GI_Default.PuzzlePiece2` _asgi_default))
  (if (and (== _puzzlepiece1 false) (== _puzzlepiece2 false))
    _
    (elif (and (== _puzzlepiece1 true) (== _puzzlepiece2 false))
      (`SceneComponent.SetHiddenInGame` (`self.keyPiece1`) false false)
      (`SceneComponent.SetVisibility` (`self.keyPiece1`) true false)
      (elif (and (== _puzzlepiece1 false) (== _puzzlepiece2 true))
        (`SceneComponent.SetHiddenInGame` _keypiece2_2 false false)
        (`SceneComponent.SetVisibility` _keypiece2_2 true false)
        (elif (and (== _puzzlepiece1 true) (== _puzzlepiece2 true))
          (`SceneComponent.SetHiddenInGame` _keypiece1 false false)
          (`SceneComponent.SetHiddenInGame` _keypiece2 false false)
          (`SceneComponent.SetVisibility` _keypiece1 true false)
          (`SceneComponent.SetVisibility` _keypiece2 true false)
          (`SceneComponent.SetVisibility` (`self.ChestKey`) true false)
          (`self.Open Drawer`))))))

(event `Open Drawer`
  (`/Engine/EditorBlueprintResources/StandardMacros.DoOnce` false
    (:`Completed`
      (bind (_direction _rotate) (`Timeline|Timeline` :!via `PlayFromStart`)
        (:`Update`
          (`SceneComponent.K2_SetRelativeLocation` (`self.Box`) (`KismetMathLibrary.MakeVector` 0.0 _rotate -9.0) false false))))))

(fn `OnInteracted`
  (params (`Component Hit` :type "PrimitiveComponent Object Reference"))
  (returns (`Interactable Actor` :type "Actor Object Reference") (`Interaction Type` :type "/Game/Data/Enums/Enum_InteractionType Enum") (ItemInfo :type "/Game/Data/ItemData/STR_ItemInfo Structure"))
  (`self.Interacted`)
  (return null "NewEnumerator5"))

(fn `OnPawnChanged`
  (returns (`Pawn Enum` :type "/Game/Data/Enums/Enum_PossessedPawn Enum"))
  (return "NewEnumerator0"))

(fn `UserConstructionScript`)