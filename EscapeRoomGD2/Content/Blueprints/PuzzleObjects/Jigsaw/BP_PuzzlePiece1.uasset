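; BP_PuzzlePiece1 is an interactable jigsaw puzzle piece whose pickup is recorded on the game instance.
; Its Interacted event runs through a FlipFlop: the first interaction sets the PuzzlePiece1 flag on GI_Default, and the second destroys the actor.
; BeginPlay, overlap and Tick are disabled stubs, and the construction script only calls its parent.
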(event `self.Interacted`
  (`/Engine/EditorBlueprintResources/StandardMacros.FlipFlop`
    (:`A`
      (bind _asgi_default (cast `/Game/Levels/LevelData/GI_Default` (`GameplayStatics.GetGameInstance`)))
      (set `/Game/Levels/LevelData/GI_Default.PuzzlePiece1` true _asgi_default))
    (:`B`
      (`self.K2_DestroyActor`))))

(fn `UserConstructionScript`
  (`parent.UserConstructionScript`))