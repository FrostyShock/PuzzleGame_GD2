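; BP_Chest is an interactable puzzle chest that highlights both halves through custom depth when focused.
; On its first interaction, a timeline shows, inserts and turns the key, then a second timeline rotates the lid open.
; The GameInstance JigsawKey check is disconnected, so the chest opens without requiring that key.
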(event `/Game/Data/Interfaces/BPI_PuzzleGame.On Focused`
  (params (Focused :type Boolean) (Component :type "PrimitiveComponent Object Reference"))
  (`PrimitiveComponent.SetRenderCustomDepth` (`self.chestBottom`) Focused)
  (`PrimitiveComponent.SetRenderCustomDepth` (`self.chestTop`) Focused))

(event `Interacted`
  (bind _key (`self.key`))
  (`/Engine/EditorBlueprintResources/StandardMacros.DoOnce` false
    (:`Completed`
      (`SceneComponent.SetVisibility` (`self.key`) true false)
      (bind (_direction _key_insert _rotation) (`Timeline|KeyTurning` :!via `PlayFromStart`)
        (:`Update`
          (`SceneComponent.K2_SetRelativeLocation` _key _key_insert false false)
          (`SceneComponent.K2_SetRelativeRotation` _key (`KismetMathLibrary.MakeRotator` 0.0 _rotation) false false))
        (:`Finished`
          (bind (_direction_2 _lid_rotation) (`Timeline|Lid Opening` :!via `PlayFromStart`)
            (:`Update`
              (`SceneComponent.K2_SetRelativeRotation` (`self.chestTop`) (`KismetMathLibrary.MakeRotator` _lid_rotation) false false))))))))

(fn `OnInteracted`
  (params (`Component Hit` :type "PrimitiveComponent Object Reference"))
  (returns (`Interactable Actor` :type "Actor Object Reference") (`Interaction Type` :type "/Game/Data/Enums/Enum_InteractionType Enum") (ItemInfo :type "/Game/Data/ItemData/STR_ItemInfo Structure"))
  (`self.Interacted`)
  (return null "NewEnumerator5"))

(fn `OnPawnChanged`
  (returns (`Pawn Enum` :type "/Game/Data/Enums/Enum_PossessedPawn Enum"))
  (return "NewEnumerator0"))

(fn `UserConstructionScript`)