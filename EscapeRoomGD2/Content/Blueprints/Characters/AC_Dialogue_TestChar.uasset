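; Dialogue component for the Bartender, who greets the player and gives puzzle hints in the bar.
; The Dialogue override builds a branching tree of AddDialogue calls, each switching on dialogue state and chosen option.
; Asking for help reads the Riddle1Clue and PerspClue flags from GI_Default to pick one of four hint sub-trees, up to the puzzle solution.
; Endings clear progress and close the conversation; only tree index 0 is implemented.
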(fn `Dialogue`
  (`parent.Dialogue`)
  (switch `int` (`self.DialogueTreeIndex`)
    (:`0`
      (bind (_dialoguestate _option_index) (`self.AddDialogue` "Bartender" "Welcome to my wonderful bar; we hope you enjoy your stay. You may be here for a while." (`|MakeArray` "What do you mean by that?" "Whatever, bye." :!type "Text")))
      (switch `/Game/Data/Enums/Enum_DialogueState` _dialoguestate
        (:`NewEnumerator0`
          (switch `int` _option_index
            (:`0`
              (bind (_dialoguestate_2 _option_index_2) (`self.AddDialogue` "Bartender" "Well, you see, most wayward souls who find themselves in this bar are on a one-way trip. What brings them here is of little import to me. Maybe you'll find some clues to find your way on through." (`|MakeArray` "That's eerie. Can you help me?" "See ya." :!type "Text")))
              (switch `/Game/Data/Enums/Enum_DialogueState` _dialoguestate_2
                (:`NewEnumerator0`
                  (switch `int` _option_index_2
                    (:`0`
                      ; Puzzle Hints
                      (bind _asgi_default (cast `/Game/Levels/LevelData/GI_Default` (`GameplayStatics.GetGameInstance`)))
                      (if (and (not (`/Game/Levels/LevelData/GI_Default.Riddle1Clue` _asgi_default)) (not (`/Game/Levels/LevelData/GI_Default.PerspClue` _asgi_default)))
                        (bind (_dialoguestate_3 _option_index_3) (`self.AddDialogue` "Bartender" "I suppose a tip wouldn't hurt. Check around for conspicuous items or flickering lights. Someone seems to have tampered with the power." (`|MakeArray` "The lights?" "Conspicuous items?" :!type "Text")))
                        (switch `/Game/Data/Enums/Enum_DialogueState` _dialoguestate_3
                          (:`NewEnumerator0`
                            (switch `int` _option_index_3
                              (:`0`
                                (bind _dialoguestate_4 (`self.AddDialogue` "Bartender" "Yes, one of the lights by the tables seems to be having an issue right now. " (`|MakeArray` "Oh, okay." :!type "Text")))
                                (switch `/Game/Data/Enums/Enum_DialogueState` _dialoguestate_4
                                  (:`NewEnumerator0`
                                    (`self.ClearDialogueProgress`)
                                    (`self.CloseConversation`))))
                              (:`1`
                                (bind _dialoguestate_5 (`self.AddDialogue` "Bartender" "Down in the lounge, somebody seems to have left a telescope near the window. I certainly didn't place it there. " (`|MakeArray` "Okay." :!type "Text")))
                                (switch `/Game/Data/Enums/Enum_DialogueState` _dialoguestate_5
                                  (:`NewEnumerator0`
                                    (`self.ClearDialogueProgress`)
                                    (`self.CloseConversation`)))))))
                        (elif (and (`/Game/Levels/LevelData/GI_Default.Riddle1Clue` _asgi_default) (not (`/Game/Levels/LevelData/GI_Default.PerspClue` _asgi_default)))
                          (bind (_dialoguestate_6 _option_index_4) (`self.AddDialogue` "Bartender" "Oh you found a riddle. What could it mean?" (`|MakeArray` "I figured out the riddle, what should I do about it?" "Are you still yapping?." :!type "Text")))
                          (switch `/Game/Data/Enums/Enum_DialogueState` _dialoguestate_6
                            (:`NewEnumerator0`
                              (switch `int` _option_index_4
                                (:`0`
                                  (bind (_dialoguestate_7 _option_index_5) (`self.AddDialogue` "Bartender" "I hope you've found the other clues as well." (`|MakeArray` "Oh, I'll do that." "Could you help me?" :!type "Text")))
                                  (switch `/Game/Data/Enums/Enum_DialogueState` _dialoguestate_7
                                    (:`NewEnumerator0`
                                      (switch `int` _option_index_5
                                        (:`0`
                                          (`self.ClearDialogueProgress`)
                                          (`self.CloseConversation`))
                                        (:`1`
                                          (bind _dialoguestate_8 (`self.AddDialogue` "Bartender" "Try checking the lounge. Somebody seems to have left a telescope. " (`|MakeArray` "Oh, I'll do that." :!type "Text")))
                                          (switch `/Game/Data/Enums/Enum_DialogueState` _dialoguestate_8
                                            (:`NewEnumerator0`
                                              (`self.ClearDialogueProgress`)
                                              (`self.CloseConversation`))))))))
                                (:`1`
                                  (`self.ClearDialogueProgress`)
                                  (`self.CloseConversation`)))))
                          (elif (and (not (`/Game/Levels/LevelData/GI_Default.Riddle1Clue` _asgi_default)) (`/Game/Levels/LevelData/GI_Default.PerspClue` _asgi_default))
                            (bind (_dialoguestate_9 _option_index_6) (`self.AddDialogue` "Bartender" "So you've seen into the void? What did you think?" (`|MakeArray` "I think I understood it." "I'm not sure what it meant." "I've seen better." :!type "Text")))
                            (switch `/Game/Data/Enums/Enum_DialogueState` _dialoguestate_9
                              (:`NewEnumerator0`
                                (switch `int` _option_index_6
                                  (:`0`
                                    (bind (_dialoguestate_10 _option_index_7) (`self.AddDialogue` "Bartender" "Does anyone truly understand it? Though, you do seem quite astute." (`|MakeArray` "See ya around." "What did you call me?" :!type "Text")))
                                    (switch `/Game/Data/Enums/Enum_DialogueState` _dialoguestate_10
                                      (:`NewEnumerator0`
                                        (switch `int` _option_index_7
                                          (:`0`
                                            (`self.ClearDialogueProgress`)
                                            (`self.CloseConversation`))
                                          (:`1`
                                            (bind _dialoguestate_11 (`self.AddDialogue` "Bartender" "Oh, I guess I was wrong." (`|MakeArray` "[End Dialogue.]" :!type "Text")))
                                            (switch `/Game/Data/Enums/Enum_DialogueState` _dialoguestate_11
                                              (:`NewEnumerator0`
                                                (`self.ClearDialogueProgress`)
                                                (`self.CloseConversation`))))))))
                                  (:`1`
                                    (bind (_dialoguestate_12 _option_index_8) (`self.AddDialogue` "Bartender" "Maybe you should find another clue? Perhaps that might elucidate your next steps." (`|MakeArray` "Like what?" "See ya around!" :!type "Text")))
                                    (switch `/Game/Data/Enums/Enum_DialogueState` _dialoguestate_12
                                      (:`NewEnumerator0`
                                        (switch `int` _option_index_8
                                          (:`0`
                                            (bind (_dialoguestate_13 _option_index_9) (`self.AddDialogue` "Bartender" "Must I spell it out for you? Oh well. Perhaps check the napkins around the tables." (`|MakeArray` "[End Dialogue.]" :!type "Text")))
                                            (switch `/Game/Data/Enums/Enum_DialogueState` _dialoguestate_13
                                              (:`NewEnumerator0`
                                                (switch `int` _option_index_9
                                                  (:`0`
                                                    (`self.ClearDialogueProgress`)
                                                    (`self.CloseConversation`))))))
                                          (:`1`
                                            (`self.ClearDialogueProgress`)
                                            (`self.CloseConversation`))))))
                                  (:`2`
                                    (bind _dialoguestate_14 (`self.AddDialogue` "Bartender" "Oh, certainly.Maybe I'll take you there." (`|MakeArray` "Oop" :!type "Text")))
                                    (switch `/Game/Data/Enums/Enum_DialogueState` _dialoguestate_14
                                      (:`NewEnumerator0`
                                        (`self.ClearDialogueProgress`)
                                        (`self.CloseConversation`)))))))
                            (elif (and (`/Game/Levels/LevelData/GI_Default.Riddle1Clue` _asgi_default) (`/Game/Levels/LevelData/GI_Default.PerspClue` _asgi_default))
                              (bind (_dialoguestate_15 _option_index_10) (`self.AddDialogue` "Bartender" "It seems you've found at least two of the clues. Well done. What might I help you with now?" (`|MakeArray` "I'm not sure what my next step is." "Eh nevermind." :!type "Text")))
                              (switch `/Game/Data/Enums/Enum_DialogueState` _dialoguestate_15
                                (:`NewEnumerator0`
                                  (switch `int` _option_index_10
                                    (:`0`
                                      (bind (_dialoguestate_16 _option_index_11) (`self.AddDialogue` "Bartender" "Perhaps there is some meaning to the symbols behind me; though, I can't make heads or tails of it. " (`|MakeArray` "Oh I think I get it now." "I really, really do not understand what to do next. (Solution to Puzzle)" :!type "Text")))
                                      (switch `/Game/Data/Enums/Enum_DialogueState` _dialoguestate_16
                                        (:`NewEnumerator0`
                                          (switch `int` _option_index_11
                                            (:`0`
                                              (bind _dialoguestate_17 (`self.AddDialogue` "Bartender" "Fantastic! Good luck!" (`|MakeArray` "[End Dialogue]" :!type "Text")))
                                              (switch `/Game/Data/Enums/Enum_DialogueState` _dialoguestate_17
                                                (:`NewEnumerator0`
                                                  (`self.ClearDialogueProgress`)
                                                  (`self.CloseConversation`))))
                                            (:`1`
                                              (bind _dialoguestate_18 (`self.AddDialogue` "Bartender" "Count the number of symbols that match the shadow on the ceiling. " (`|MakeArray` "Thank you. " :!type "Text")))
                                              (switch `/Game/Data/Enums/Enum_DialogueState` _dialoguestate_18
                                                (:`NewEnumerator0`
                                                  (`self.ClearDialogueProgress`)
                                                  (`self.CloseConversation`))))))))
                                    (:`1`
                                      (`self.ClearDialogueProgress`)
                                      (`self.CloseConversation`)))))
                              (elif true
                                _))))))
                    (:`1`
                      (bind _dialoguestate_19 (`self.AddDialogue` "Bartender" "Come back to see me if you need help. " (`|MakeArray` "[Exit]" :!type "Text")))
                      (switch `/Game/Data/Enums/Enum_DialogueState` _dialoguestate_19
                        (:`NewEnumerator0`
                          (`self.ClearDialogueProgress`)
                          (`self.CloseConversation`))))))))
            (:`1`
              (bind _dialoguestate_20 (`self.AddDialogue` "Bartender" "Come back to see me if you need help. " (`|MakeArray` "[Exit]" :!type "Text")))
              (switch `/Game/Data/Enums/Enum_DialogueState` _dialoguestate_20
                (:`NewEnumerator0`
                  (`self.ClearDialogueProgress`)
                  (`self.CloseConversation`))))))))))