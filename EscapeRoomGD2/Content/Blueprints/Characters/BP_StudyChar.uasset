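; BP_StudyChar is an interactable study character that holds a conversation with the player.
; Interaction opens the ACDialogueStudyChar conversation through a DoOnce and switches the animation state.
; Closing it restores the player controller's default mapping and animation state, then re-arms the DoOnce.
; When the player enters ActivationVolume, the sweep normal's direction decides whether ClueGuyRigged is activated or deactivated.
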(event `Begin Dialogue`
  (`/Engine/EditorBlueprintResources/StandardMacros.DoOnce` false :!label _label
    (:`Completed`
      (`/Game/Data/Components/AC_DialogueComponent.OpenConversation` (`self.AC_Dialogue_StudyChar`))
      (set `self.Anim States` "NewEnumerator2"))))

(event `self.Conversation Closed`
  (bind _asbp_player_controller (cast `/Game/Player/BP_PlayerController` (`GameplayStatics.GetPlayerController` 0)))
  (`/Game/Player/BP_PlayerController.Default Player Map Change` _asbp_player_controller)
  (set `self.Anim States` "NewEnumerator0")
  (goto _label :!via `Reset`))

(event `self.Activation Volume.OnComponentBeginOverlap`
  (params (OverlappedComponent :type "PrimitiveComponent Object Reference") (OtherActor :type "Actor Object Reference") (OtherComp :type "PrimitiveComponent Object Reference") (OtherBodyIndex :type Integer) (bFromSweep :type Boolean) (SweepResult :type "HitResult Structure (by ref)"))
  (bind _clueguyrigged (`self.clueGuyRigged`))
  (if (== OtherActor (`GameplayStatics.GetPlayerPawn` 0))
    (if (== (`.Normal` (`GameplayStatics.BreakHitResult` SweepResult)) (0.0 -1.0 0.0) :`ErrorTolerance` 0.3)
      (`ActorComponent.SetActive` _clueguyrigged false true)
      (else
        (`ActorComponent.SetActive` _clueguyrigged true true)))))

(fn `OnInteracted`
  (params (`Component Hit` :type "PrimitiveComponent Object Reference"))
  (returns (`Interactable Actor` :type "Actor Object Reference") (`Interaction Type` :type "/Game/Data/Enums/Enum_InteractionType Enum") (ItemInfo :type "/Game/Data/ItemData/STR_ItemInfo Structure"))
  (`self.Begin Dialogue`)
  (return self "NewEnumerator2"))

(fn `OnPawnChanged`
  (returns (`Pawn Enum` :type "/Game/Data/Enums/Enum_PossessedPawn Enum"))
  (return "NewEnumerator0"))

(fn `UserConstructionScript`)