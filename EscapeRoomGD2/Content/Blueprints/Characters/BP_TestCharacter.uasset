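; BP_TestCharacter is a test NPC that can be interacted with to open a dialogue.
; OnInteracted fires BeginDialogue, which uses a DoOnce to open the conversation on its dialogue component; ConversationClosed restores the player controller's default player map and resets the gate.
; On BeginPlay a looping timer, with its interval randomised once, flips AnimState between two values to alternate animations.
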(event `Begin Dialogue`
  (`/Engine/EditorBlueprintResources/StandardMacros.DoOnce` false :!label _label
    (:`Completed`
      (`/Game/Data/Components/AC_DialogueComponent.OpenConversation` (`self.AC_Dialogue_TestChar`)))))

(event `/Game/Data/Interfaces/BPI_PuzzleGame.Conversation Closed`
  (bind _asbp_player_controller (cast `/Game/Player/BP_PlayerController` (`GameplayStatics.GetPlayerController` 0)))
  (`/Game/Player/BP_PlayerController.Default Player Map Change` _asbp_player_controller)
  (goto _label :!via `Reset`))

(event `self.ReceiveBeginPlay`
  (`KismetSystemLibrary.K2_SetTimerDelegate` (delegate `Loop anim`) (`KismetMathLibrary.RandomFloatInRange` 1.6 6.0) true))

(event `Loop anim`
  (`/Engine/EditorBlueprintResources/StandardMacros.FlipFlop`
    (:`A`
      (set `self.anim State` 1))
    (:`B`
      (set `self.anim State` 0))))

(fn `OnInteracted`
  (params (`Component Hit` :type "PrimitiveComponent Object Reference"))
  (returns (`Interactable Actor` :type "Actor Object Reference") (`Interaction Type` :type "/Game/Data/Enums/Enum_InteractionType Enum") (ItemInfo :type "/Game/Data/ItemData/STR_ItemInfo Structure"))
  (`self.Begin Dialogue`)
  (return self "NewEnumerator2"))

(fn `OnPawnChanged`
  (returns (`Pawn Enum` :type "/Game/Data/Enums/Enum_PossessedPawn Enum"))
  (return "NewEnumerator0"))

(fn `UserConstructionScript`)