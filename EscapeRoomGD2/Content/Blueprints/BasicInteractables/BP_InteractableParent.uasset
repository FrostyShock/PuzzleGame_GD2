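; BP_InteractableParent is a base actor for basic interactables that records its original transform in the construction script.
; OnInteracted fires the Interacted event, then returns the actor itself with an interaction type; OnPawnChanged only returns an enum value.
; The default Interacted alternates through a FlipFlop: the first branch does nothing, and the second teleports the actor back to its stored transform.
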(event `self.ReceiveBeginPlay`)

(event `Interacted`
  (`/Engine/EditorBlueprintResources/StandardMacros.FlipFlop`
    (:`B`
      (`self.K2_SetActorTransform` self (`self.Original Position`) false true))))

(fn `OnInteracted`
  (returns (`Interactable Actor` :type "Actor Object Reference") (`Interaction Type` :type "/Game/Data/Enums/Enum_InteractionType Enum"))
  (`self.Interacted`)
  (return self "NewEnumerator0"))

(fn `OnPawnChanged`
  (returns (`Pawn Enum` :type "/Game/Data/Enums/Enum_PossessedPawn Enum"))
  (return "NewEnumerator0"))

(fn `UserConstructionScript`
  (set `self.Original Position` (`self.GetTransform` self)))