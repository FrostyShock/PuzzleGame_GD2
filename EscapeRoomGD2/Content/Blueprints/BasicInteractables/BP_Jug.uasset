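; BP_Jug is an interactable jug that toggles between a first-person state and a return to its original spot.
; Interacting alternates between rendering the mesh as a first-person primitive and playing a Timeline that lerps the actor to its construction-time transform, clearing that flag.
; Focus toggles custom depth on the component.
; OnInteracted triggers the toggle and returns the jug's interaction type and item info.
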(event `self.ReceiveBeginPlay`)

(event `Interacted`
  (bind _objmesh (`self.ObjMesh`))
  (`/Engine/EditorBlueprintResources/StandardMacros.FlipFlop`
    (:`A`
      (`PrimitiveComponent.SetFirstPersonPrimitiveType` _objmesh "FirstPerson"))
    (:`B`
      (bind (_direction _lerp_value) (`Timeline|Timeline` :!via `PlayFromStart`)
        (:`Update`
          (bind (_returnvalue_location _returnvalue_rotation _returnvalue_scale) (`KismetMathLibrary.BreakTransform` (`KismetMathLibrary.TLerp` (`self.GetTransform`) (`self.Original Position`) _lerp_value)))
          (`self.K2_SetActorTransform` self (`KismetMathLibrary.MakeTransform` _returnvalue_location _returnvalue_rotation _returnvalue_scale) false true)
          (`PrimitiveComponent.SetFirstPersonPrimitiveType` _objmesh "None"))))))

(event `self.On Focused`
  (params (Focused :type Boolean) (Component :type "PrimitiveComponent Object Reference"))
  (`PrimitiveComponent.SetRenderCustomDepth` Component Focused))

(event `/Game/Data/Interfaces/BPI_PuzzleGame.On Pickup`
  (params (`Target Component` :type "PrimitiveComponent Object Reference")))

(fn `OnInteracted`
  (params (`Component Hit` :type "PrimitiveComponent Object Reference"))
  (returns (`Interactable Actor` :type "Actor Object Reference") (`Interaction Type` :type "/Game/Data/Enums/Enum_InteractionType Enum") (ItemInfo :type "/Game/Data/ItemData/STR_ItemInfo Structure"))
  (`self.Interacted`)
  (return self "NewEnumerator0" (`self.ItemInfo`)))

(fn `OnPawnChanged`
  (returns (`Pawn Enum` :type "/Game/Data/Enums/Enum_PossessedPawn Enum"))
  (return "NewEnumerator0"))

(fn `UserConstructionScript`
  (set `self.Original Position` (`self.GetTransform` self)))